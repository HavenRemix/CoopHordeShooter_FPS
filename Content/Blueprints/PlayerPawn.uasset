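; PlayerPawn is the player's pawn Blueprint, handling local HUD setup, in-game menu access and a melee attack.
; On BeginPlay, the locally controlled pawn creates crosshair, health indicator and main HUD widgets and sets default mouse sensitivities.
; The menu input opens a widget with UI-only input and a visible cursor.
; Melee damages every actor overlapping its Box; an alternative radial-damage node is left disconnected.
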(event `self.ReceiveBeginPlay`
  (if (`self.IsLocallyControlled`)
    (`|ExecutionSequence`
      (:`then_0`
        (bind _returnvalue (`|CreateWidget` "/Game/UI/WBP_Crosshair.WBP_Crosshair_C"))
        (`UserWidget.AddToViewport` _returnvalue 0))
      (:`then_1`
        (bind _returnvalue_2 (`|CreateWidget` "/Game/UI/WBP_HealthIndicator.WBP_HealthIndicator_C"))
        (`UserWidget.AddToViewport` _returnvalue_2 0))
      (:`then_2`
        (set `self.MouseXSens` 1.0)
        (set `self.MouseYSens` 1.0)
        (set `self.MouseTargetingSens` 0.6))
      (:`then_3`
        (bind _returnvalue_3 (`|CreateWidget` "/Game/UI/WBP_MainHUD.WBP_MainHUD_C"))
        (`UserWidget.AddToViewport` _returnvalue_3 0)))))

(event `InputAction|InGameMenu`
  (params (Key :type "Key Structure"))
  (:`Pressed`
    (bind _returnvalue (`|CreateWidget` "/Game/UI/Menu/WBP_InGameMenu.WBP_InGameMenu_C"))
    (`UserWidget.AddToViewport` _returnvalue 0)
    (`WidgetBlueprintLibrary.SetInputMode_UIOnlyEx` (`GameplayStatics.GetPlayerController` 0) null)
    (set `PlayerController.bShowMouseCursor` true (`GameplayStatics.GetPlayerController` 0))))

(event `InputAction|Melee`
  (params (Key :type "Key Structure"))
  (:`Pressed`
    (for _array_element (`PrimitiveComponent.GetOverlappingActors` (`self.Box`) null)
      (`GameplayStatics.ApplyDamage` _array_element 150.0 (`self.GetInstigatorController`) self))))

(fn `UserConstructionScript`)